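; Actor component that lets its owner interact with objects in view and carry physics objects.
; BeginPlay creates the crosshair widget and finds the owner's camera; Tick line-traces forward for BPI_Interaction actors or physics-simulating objects, updating the crosshair.
; Interacting sends InteractMessage and starts a grab if the actor simulates physics.
; Grabbed components, optionally filtered by GrabTag, follow a point ahead of the camera through velocity steering rather than a physics handle.
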(event Custom|interact
  (bind _interactactorref (Variables|PrivateVar|GetinteractActorRef))
  ;[1 1 1] Interact
  (Utilities|IsValid _interactactorref
    (:Is%20Valid
      (Utilities|FlowControl|DoOnce false
        (:Completed
          (Class|BPIInteraction|Interact(Message) _interactactorref)
          (Variables|PrivateVar|SetisInteracting (Physics|IsSimulatingPhysics (Variables|/Script/Engine.Actor|GetRootComponent _interactactorref) "None")))))))

(event Custom|BreakCameraLoop
  ;[1 1 1] FindPlayerCamera
  (Utilities|Array|ForEachLoopwithBreak (Components|GetChildrenComponents (Variables|/Script/Engine.Actor|GetRootComponent (Components|GetOwner)) true)) ; enters at Break
)

(event Custom|stopInteraction
  (bind _interactactorref (Variables|PrivateVar|GetinteractActorRef))
  ;[1 1 1] Interact
  (Variables|PrivateVar|SetisInteracting false)
  (Utilities|FlowControl|DoOnce false) ; enters at Reset
)

(event EventBeginPlay
  (bind _crosshair (Variables|Crosshair|GetcrossHair))
  ;[1 1 1] SetCrossHair
  (if (Utilities|IsValidClass _crosshair)
    (bind _returnvalue (UserInterface|CreateWidget _crosshair))
    (bind _output_get (Variables|PrivateVar|SetcrossHairRef _returnvalue))
    (UserInterface|Viewport|AddtoViewport _output_get 0)
    (Class|BPIInteraction|ShowCrosshair(Message) _output_get (Variables|Crosshair|GetalwaysShowCrosshair)))
  ;[1 1 1] FindPlayerCamera
  (bind _array_element (Utilities|Array|ForEachLoopwithBreak (Components|GetChildrenComponents (Variables|/Script/Engine.Actor|GetRootComponent (Components|GetOwner)) true))
    (:LoopBody
      (if (== _array_element "/Script/Engine.CameraComponent")
        (Variables|PrivateVar|SetcameraRef _array_element)
        (CallFunction|BreakCameraLoop)))
    (:Completed
      ;[1 0 0] DEBUG
      (Utilities|IsValid (Variables|PrivateVar|GetcameraRef)
        (:Is%20Not%20Valid
          (Development|PrintString "No Camera Detected"))))))

(event EventTick
  (params (DeltaSeconds :type Float%20%28single-precision%29))
  (bind _cameraref (Variables|PrivateVar|GetcameraRef))
  (bind _returnvalue (Transformation|GetWorldLocation _cameraref))
  ;[1 1 1] UpdateLocation
  (if (Variables|PrivateVar|GetisInteracting)
    (Utilities|IsValid (Variables|PrivateVar|GetinteractComponentRef)
      (:Is%20Valid
        (|SetActorLoc)))
    (else
      ;[1 1 1] lineTrace
      (bind (_outhit _returnvalue_2) (Collision|LineTraceByChannel _returnvalue (+ _returnvalue (* (Math|Vector|GetForwardVector _cameraref) (Variables|Grab|GetinteractDistance))) (Variables|Grab|GetinteractChannel) false 0 "None"))
      ;[1 1 1] FindActor
      (if _returnvalue_2
        (if (!= (.HitActor (Collision|BreakHitResult _outhit)) (Variables|PrivateVar|GetinteractActorRef))
          (Variables|PrivateVar|SetinteractActorRef (.HitActor (Collision|BreakHitResult _outhit))))
        (if (Utilities|DoesObjectImplementInterface (Variables|PrivateVar|GetinteractActorRef) "/Game/Interaction/BPI_Interaction.BPI_Interaction_C")
          ;[1 1 1] SetCrossHair
          (if (not (Variables|Crosshair|GetalwaysShowCrosshair)) :!label _label
            (Class|BPIInteraction|ShowCrosshair(Message) (Variables|PrivateVar|GetcrossHairRef) true)
            (goto _label_2 Reset))
          (else
            ;[1 1 1] setComponentRef
            (if (Physics|IsSimulatingPhysics (Variables|/Script/Engine.Actor|GetRootComponent (Variables|PrivateVar|GetinteractActorRef)) "None")
              (Variables|PrivateVar|SetinteractActorRef (.HitActor (Collision|BreakHitResult _outhit)))
              (Variables|PrivateVar|SetinteractComponentRef (.HitComponent (Collision|BreakHitResult _outhit)))
              (goto _label))))
        (else
          ;[1 1 1] ResetValues
          (Variables|PrivateVar|SetinteractActorRef 0)
          (Variables|PrivateVar|SetinteractComponentRef 0)
          (if (not (Variables|Crosshair|GetalwaysShowCrosshair))
            (Utilities|FlowControl|DoOnce false :!label _label_2
              (:Completed
                (Class|BPIInteraction|ShowCrosshair(Message) (Variables|PrivateVar|GetcrossHairRef) false)))))))))